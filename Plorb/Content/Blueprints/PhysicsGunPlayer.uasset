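; Player physics gun that lets the player grab, carry, throw and shove tagged objects.
; Right mouse holds an object via a PhysicsHandle; left throws the held object or applies an impulse at the aimed point.
; TraceFunction briefly disables capsule collision to line trace, enables physics on tagged hits and prints a warning for untagged ones.
; Tick keeps the handle target along the view direction at the last traced hit distance.
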(event `Key|LeftMouseButton` :overrideparent false
  (bind _physicsgrabbedcomponent (`self.PhysicsGrabbedComponent`))
  (bind _returnvalue (`KismetMathLibrary.Conv_RotatorToVector` (`self.GetControlRotation`)))
  (:`Pressed`
    (`/Engine/EditorBlueprintResources/StandardMacros.IsValid` _physicsgrabbedcomponent
      (:`Is Valid`
        (`PrimitiveComponent.AddImpulse` _physicsgrabbedcomponent (* _returnvalue (`self.ThrowImpulse`)) "None" false)
        (`PhysicsHandleComponent.ReleaseComponent` (`self.Physics Handle`))
        (set `self.PhysicsGrabbedComponent` null))
      (:`Is Not Valid`
        (bind (_impact_point _hit_component _bone_name _impulse) (`self.Trace Function` _returnvalue))
        (`PrimitiveComponent.AddImpulseAtLocation` _hit_component _impulse _impact_point _bone_name)))))

(event `Key|RightMouseButton` :consume false :overrideparent false
  (bind _physics_handle (`self.Physics Handle`))
  (:`Pressed`
    (bind (_impact_point _hit_component _bone_name) (`self.Trace Function` (0.0 0.0 0.0)))
    (`PhysicsHandleComponent.GrabComponent` _physics_handle _hit_component _bone_name _impact_point false)
    (set `self.PhysicsGrabbedComponent` _hit_component))
  (:`Released`
    (`/Engine/EditorBlueprintResources/StandardMacros.IsValid` (`self.PhysicsGrabbedComponent`)
      (:`Is Valid`
        (`PhysicsHandleComponent.ReleaseComponent` _physics_handle)
        (set `self.PhysicsGrabbedComponent` null)))))

(event `self.ReceiveTick`
  (params (DeltaSeconds :type "Float (single-precision)"))
  (set `self.StartLoc` (`KismetMathLibrary.MakeVector` (+ (.x (`self.K2_GetActorLocation` (`GameplayStatics.GetPlayerCharacter` 0))) 1.0) (.y (`self.K2_GetActorLocation` (`GameplayStatics.GetPlayerCharacter` 0))) (+ (.z (`self.K2_GetActorLocation` (`GameplayStatics.GetPlayerCharacter` 0))) 50.0)))
  (`PhysicsHandleComponent.SetTargetLocation` (`self.Physics Handle`) (+ (`self.StartLoc`) (* (`KismetMathLibrary.Conv_RotatorToVector` (`self.GetControlRotation`)) (`self.HitDistance`)))))

(fn `Trace Function`
  (params (`Controller Aim` :type "Object.Vector Structure"))
  (returns (`Impact Point` :type "Object.Vector Structure") (`Hit Component` :type "PrimitiveComponent Object Reference") (`Bone Name` :type Name) (Impulse :type "Object.Vector Structure"))
  (bind _starttrace (`self.StartTrace`))
  (set `self.StartTrace` (`KismetMathLibrary.MakeVector` (+ (.x (`self.K2_GetActorLocation` (`GameplayStatics.GetPlayerCharacter` 0))) 1.0) (.y (`self.K2_GetActorLocation` (`GameplayStatics.GetPlayerCharacter` 0))) (+ (.z (`self.K2_GetActorLocation` (`GameplayStatics.GetPlayerCharacter` 0))) 50.0)))
  (set `self.EndTrace` (+ (`self.StartTrace`) (* (`KismetMathLibrary.Conv_RotatorToVector` (`self.GetControlRotation`)) 10000.0)))
  (`PrimitiveComponent.SetCollisionEnabled` (`Character.CapsuleComponent` (`GameplayStatics.GetPlayerCharacter` 0)) "NoCollision")
  (bind _outhit (`KismetSystemLibrary.LineTraceSingle_DEPRECATED` _starttrace (`self.EndTrace`) "ECC_WorldDynamic"))
  (`PrimitiveComponent.SetCollisionEnabled` (`Character.CapsuleComponent` (`GameplayStatics.GetPlayerCharacter` 0)) "QueryAndPhysics")
  (bind (_location _normal _impactpoint _impactnormal _physmat _hitactor _hitcomponent _hitbonename) (`GameplayStatics.BreakHitResult` _outhit))
  (`/Engine/EditorBlueprintResources/StandardMacros.IsValid` _hitactor
    (:`Is Valid`
      (set `self.HitDistance` (`KismetMathLibrary.VSize` (- _location _starttrace)))
      (if (`self.ActorHasTag` _hitactor (`self.TagName`))
        (`PrimitiveComponent.SetSimulatePhysics` _hitcomponent true)
        (return _impactpoint _hitcomponent _hitbonename (* `Controller Aim` (`self.Impulse`)))
        (else
          (bind _returnvalue (`KismetSystemLibrary.GetDisplayName` _hitactor))
          (if (`KismetStringLibrary.NotEqual_StrStr` _returnvalue)
            (`KismetSystemLibrary.PrintString` (`KismetStringLibrary.Concat_StrStr` (`KismetStringLibrary.Concat_StrStr` (`KismetStringLibrary.Concat_StrStr` _returnvalue " cannot be moved. MISSING \"") (`KismetStringLibrary.Conv_NameToString` (`self.TagName`))) "\" Tag!") true false)))))))

(fn `UserConstructionScript`)